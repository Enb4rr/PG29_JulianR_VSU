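; Actor component that tracks the score for a target game and signals game over once the maximum score is reached.
; It uses gameplay message channels: a start-timer message initializes the UI score board and begins listening for add-to-score messages.
; Each score message adds to the total, broadcasts game over at or above the max, then pushes the new score to the UI board.
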(event `self.ReceiveBeginPlay`
  ;[0 0 0 0.5] Listens for target's game starting event
  (`|AsyncAction_ListenForGameplayMessages` (struct :`TagName` "Game.StartTimer") "/Game/Blueprints/Structs/S_Bool.S_Bool"
    (:`OnMessageReceived`
      (`self.Event StartTargetGame`))))

(event `Event StartTargetGame`
  ;[0 0 0 0.5] Updates Score table, wait for score events
  (`GameplayMessageSubsystem.K2_BroadcastMessage` (subsystem `GameplayMessageSubsystem`) (struct :`TagName` "UI.Score.InitializeBoard") (make `/Game/Blueprints/Structs/S_Int` (`self._maxScore`)))
  (bind (_asynctaskproxy _actualchannel _payload) (`|AsyncAction_ListenForGameplayMessages` (struct :`TagName` "Game.Score.AddToScore") "/Game/Blueprints/Structs/S_Int.S_Int")
    (:`OnMessageReceived`
      (`self.AddToScore` (`.Value_2_00F162FE4079024DE23AF599766CF723` (break `/Game/Blueprints/Structs/S_Int` _payload)))
      (`GameplayMessageSubsystem.K2_BroadcastMessage` (subsystem `GameplayMessageSubsystem`) (struct :`TagName` "UI.Score.UpdateBoard") (make `/Game/Blueprints/Structs/S_Int` (`self.GetScore`))))))

(fn `AddToScore`
  (params (ScoreToAdd :type Integer))
  ;[0 0 0 0.5] Adds to Score, Checks Game Win Condition
  (bind _output_get (set `self._score` (+ ScoreToAdd (`self._score`))))
  (if (>= _output_get (`self._maxScore`))
    (`GameplayMessageSubsystem.K2_BroadcastMessage` (subsystem `GameplayMessageSubsystem`) (struct :`TagName` "Game.GameOver") (make `/Game/Blueprints/Structs/S_Bool` true))))

(fn `GetMaxScore`
  (returns (_maxScore :type Integer))
  ;[0 0 0 0.5] Returns Max Score
  (return (`self._maxScore`)))

(fn `GetScore`
  (returns (_score :type Integer))
  (return (`self._score`)))