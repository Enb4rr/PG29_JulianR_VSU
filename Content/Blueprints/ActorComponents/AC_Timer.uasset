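; AC_Timer is an actor component that runs the game's countdown and signals when time is over.
; It listens for the Game.StartTimer gameplay message, then starts a looping timer.
; Each tick lowers ElapsedTime (effectively the remaining time), clamped between zero and MaxTime, and broadcasts it as an integer on UI.Timer.ElapsedTime.
; At zero it broadcasts Game.TimeOver and clears the timer.
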(event `self.ReceiveBeginPlay`
  ;[0 0 0 0.5] Subscribe to StartTimer Event
  (`|AsyncAction_ListenForGameplayMessages` (struct :`TagName` "Game.StartTimer") "/Game/Blueprints/Structs/S_Bool.S_Bool"
    (:`OnMessageReceived`
      (`self.Event StartTimer`))))

(event `Event StartTimer`
  ;[0 0 0 0.5] Start Timer on Event, broadcast endgame when time is over
  (bind _returnvalue (`KismetSystemLibrary.K2_SetTimerDelegate` (delegate `OnTimerTick`) (`self.tick`) true)))

(event `OnTimerTick`
  ;[0 0 0 0.5] Start Timer on Event, broadcast endgame when time is over
  (`self.UpdateElapsedTime`)
  (`GameplayMessageSubsystem.K2_BroadcastMessage` (subsystem `GameplayMessageSubsystem`) (struct :`TagName` "UI.Timer.ElapsedTime") (make `/Game/Blueprints/Structs/S_Int` (`KismetMathLibrary.Conv_Int64ToInt` (`KismetMathLibrary.Conv_DoubleToInt64` (`self.elapsedTime`)))))
  (if (<= (`self.elapsedTime`) 0.0)
    (`GameplayMessageSubsystem.K2_BroadcastMessage` (subsystem `GameplayMessageSubsystem`) (struct :`TagName` "Game.TimeOver") (make `/Game/Blueprints/Structs/S_Bool` false))
    (`KismetSystemLibrary.K2_ClearAndInvalidateTimerHandle` (stale `Event StartTimer` _returnvalue))))

(fn `UpdateElapsedTime`
  ;[0 0 0 0.5] Subtracts to timer
  (set `self.elapsedTime` (`KismetMathLibrary.FClamp` (- (`self.elapsedTime`) (`self.tick`)) 0.0 (`self.maxTime`))))