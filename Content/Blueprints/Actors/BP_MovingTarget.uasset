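; BP_MovingTarget is an actor that slides to a random nearby point along a single axis when play begins.
; BeginPlay randomly picks the world X or Z axis, records the start location, and GetRandomLocation offsets it along that axis within plus or minus MoveDistance.
; A timeline's alpha then lerps the actor from start to target without sweeping for collision.
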(event `self.ReceiveBeginPlay`
  (switch `int` (`KismetMathLibrary.RandomInteger` 2)
    (:`0`
      (set `self._moveAxis` (1.0 0.0 0.0)))
    (:`1`
      (set `self._moveAxis` (0.0 0.0 1.0))))
  (set `self._startLocation` (`self.K2_GetActorLocation`))
  (set `self._targetLocation` (`self.GetRandomLocation`))
  (bind (_direction _alpha) (`Timeline|MoveTarget_Timeline`)
    (:`Update`
      (`self.K2_SetActorLocation` (`KismetMathLibrary.VLerp` (`self._startLocation`) (`self._targetLocation`) _alpha)))))

(fn `GetRandomLocation`
  (returns (RandomLocation :type "Vector Structure"))
  ;[0 0 0 0.5] Returns a random location within a range
  (return (+ (`self._startLocation`) (* (`KismetMathLibrary.RandomFloatInRange` (* (`self._moveDistance`) -1.0) (`self._moveDistance`)) (`self._moveAxis`)))))

(fn `UserConstructionScript`
  (`parent.UserConstructionScript`))