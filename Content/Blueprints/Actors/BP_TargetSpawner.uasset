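; Target spawner actor that populates its SpawnArea box with common and moving targets when the game's start-timer message arrives.
; On BeginPlay it listens for the Game.StartTimer gameplay message, and each message received runs two loops that spawn a batch of BP_CommonTarget, then a batch of BP_MovingTarget.
; Both spawn functions pick a random point within the SpawnArea's scaled extent for each target.
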(event `self.ReceiveBeginPlay`
  ;[0 0 0 0.5] Wait for game start event
  (`|AsyncAction_ListenForGameplayMessages` (struct :`TagName` "Game.StartTimer") "/Game/Blueprints/Structs/S_Bool.S_Bool"
    (:`OnMessageReceived`
      (for _ (range 6)
        (`self.SpawnTarget`))
      (for _ (range 6)
        (`self.SpawnMovingTarget`)))))

(fn `SpawnMovingTarget`
  (bind _spawnarea (`self.SpawnArea`))
  ;[0 0 0 0.5] Spawns a moving target in a range
  (`|SpawnActorFromClass` "/Game/Blueprints/Actors/BP_MovingTarget.BP_MovingTarget_C" (`KismetMathLibrary.MakeTransform` (`KismetMathLibrary.RandomPointInBoundingBox` (`SceneComponent.K2_GetComponentLocation` _spawnarea) (`BoxComponent.GetScaledBoxExtent` _spawnarea))) "Undefined" "MultiplyWithRoot" null null))

(fn `SpawnTarget`
  (bind _spawnarea (`self.SpawnArea`))
  ;[0 0 0 0.5] Spawn Target BP in a range
  (`|SpawnActorFromClass` "/Game/Blueprints/Actors/BP_CommonTarget.BP_CommonTarget_C" (`KismetMathLibrary.MakeTransform` (`KismetMathLibrary.RandomPointInBoundingBox` (`SceneComponent.K2_GetComponentLocation` _spawnarea) (`BoxComponent.GetScaledBoxExtent` _spawnarea))) "Undefined" "MultiplyWithRoot" null null))

(fn `UserConstructionScript`)